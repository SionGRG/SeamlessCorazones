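; Player controller that runs a photo mode, letting the player switch to a free camera pawn, take photos and browse them.
; OpenCamera toggles between possessing a BP_PhotoCamera spawned at the current view and repossessing the character, which jumps to the camera's transform before the camera is destroyed.
; The camera's TakenPhoto event adds shots to the PhotoGallery array.
; OpenGallery toggles a UI_PhotoGallery widget of them, openable only during photo mode.
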(event `self.ReceiveBeginPlay`
  (set `self.PlayerCharacter` (`GameplayStatics.GetPlayerPawn` 0)))

(event `InputAction|OpenCamera`
  (params (Key :type "Key Structure"))
  (bind _photo_mode_camera (`self.Photo Mode Camera`))
  (:`Pressed`
    (`self.Photo Mode Camera`
      (:`then`
        (`self.UnPossess`)
        (`self.K2_SetActorTransform` (`self.PlayerCharacter`) (`self.GetTransform` (`self.Photo Mode Camera`)) false false)
        (`self.Possess` (`self.PlayerCharacter`))
        (`self.K2_DestroyActor` (`self.Photo Mode Camera`)) ; may need to save the current position of the camera so that if you moved in photo mode, u would return to that position once u exit photo mode
      )
      (:`else`
        (bind _returnvalue (`|SpawnActorFromClass` "/Game/CameraSystem/BP_PhotoCamera.BP_PhotoCamera_C" (`self.GetTransform` (`GameplayStatics.GetPlayerCameraManager` 0)) "Undefined" "OverrideRootScale" null null))
        (set `self.Photo Mode Camera` _returnvalue)
        (`self.UnPossess`)
        (`self.Possess` _photo_mode_camera)
        (add `/Game/CameraSystem/BP_PhotoCamera.TakenPhoto` _photo_mode_camera (delegate `AddToAlbum`))))))

(event `AddToAlbum`
  (params (Photo :type "TextureRenderTarget2D Object Reference"))
  (`KismetArrayLibrary.Array_Add` (`self.PhotoGallery`) Photo))

(event `InputAction|OpenGallery`
  (params (Key :type "Key Structure"))
  (:`Pressed`
    (bind _gallery (`self.Gallery`)
      (:`then`
        (`Widget.RemoveFromParent` _gallery)
        (set `self.Gallery` null))
      (:`else`
        (`self.Photo Mode Camera`
          (:`then`
            (bind _returnvalue (`|CreateWidget` "/Game/CameraSystem/UI_PhotoGallery.UI_PhotoGallery_C" null (`self.PhotoGallery`)))
            (bind _output_get (set `self.Gallery` _returnvalue))
            (`UserWidget.AddToViewport` _output_get 0))
          (:`else`))))))

(fn `UserConstructionScript`)