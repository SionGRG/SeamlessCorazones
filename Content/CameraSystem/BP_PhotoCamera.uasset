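; BP_PhotoCamera is a player-controlled photo camera that moves, looks around and takes snapshots of the scene.
; Axis inputs drive movement along the Camera's forward and right vectors and turn the controller's yaw and pitch.
; A hard-bound left mouse press creates a new render target at the configured image size for the SceneCaptureComponent2D.
; It passes that target to a new BP_PhotoDisplay widget, captures the scene and adds the widget to the viewport.
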(event `InputAxis|MoveForward`
  (params (AxisValue :type "Float (single-precision)"))
  (`self.AddMovementInput` (`SceneComponent.GetForwardVector` (`self.Camera`)) AxisValue))

(event `InputAxis|MoveRight`
  (params (AxisValue :type "Float (single-precision)"))
  (`self.AddMovementInput` (`SceneComponent.GetRightVector` (`self.Camera`)) AxisValue))

(event `InputAxis|Turn`
  (params (AxisValue :type "Float (single-precision)"))
  (`self.AddControllerYawInput` AxisValue))

(event `InputAxis|LookUp`
  (params (AxisValue :type "Float (single-precision)"))
  (`self.AddControllerPitchInput` AxisValue))

(event `Key|LeftMouseButton`
  (params (Key :type "Key Structure"))
  (:`Pressed`
    (bind _returnvalue (`KismetRenderingLibrary.CreateRenderTarget2D` (`self.CaptureImageWidth`) (`self.CaptureImageHeight`)))
    (bind _output_get (set `SceneCaptureComponent2D.TextureTarget` _returnvalue (`self.SceneCaptureComponent2D`)))
    (bind _returnvalue_2 (`|CreateWidget` "/Game/CameraSystem/BP_PhotoDisplay.BP_PhotoDisplay_C" null _output_get))
    (`SceneCaptureComponent2D.CaptureScene` (`self.SceneCaptureComponent2D`))
    (`UserWidget.AddToViewport` _returnvalue_2 0)))

(fn `UserConstructionScript`)