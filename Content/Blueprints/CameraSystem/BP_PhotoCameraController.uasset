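; BP_PhotoCameraController is a controller that toggles photo mode by switching possession between the player character and a photo camera.
; It caches the player pawn on BeginPlay, and a hardcoded C key press drives the toggle.
; Entering photo mode spawns a BP_PhotoCamera at the camera manager's transform and possesses it.
; Exiting re-possesses the character and destroys the camera, without saving its position.
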(event `self.ReceiveBeginPlay`
  (set `self.PlayerCharacter` (`GameplayStatics.GetPlayerPawn` 0)))

(event `Key|C`
  (params (Key :type "Key Structure"))
  (:`Pressed`
    (`self.Photo Mode Camera`
      (:`then`
        (`self.UnPossess`)
        (`self.Possess` (`self.PlayerCharacter`))
        (`self.K2_DestroyActor` (`self.Photo Mode Camera`)) ; may need to save the current position of the camera so that if you moved in photo mode, u would return to that position once u exit photo mode
      )
      (:`else`
        (bind _returnvalue (`|SpawnActorFromClass` "/Game/Blueprints/CameraSystem/BP_PhotoCamera.BP_PhotoCamera_C" (`self.GetTransform` (`GameplayStatics.GetPlayerCameraManager` 0)) "Undefined" "OverrideRootScale" null null))
        (set `self.Photo Mode Camera` _returnvalue)
        (`self.UnPossess`)
        (`self.Possess` (`self.Photo Mode Camera`))))))

(fn `UserConstructionScript`)