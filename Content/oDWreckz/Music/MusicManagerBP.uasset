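; Music manager Blueprint that switches between background tracks in the game.
; On BeginPlay it creates and starts every track in TrackList at zero volume, then raises the starting song to MusicVolume.
; ChangeMusicTo swaps tracks by muting the current audio component and unmuting the chosen index, so all tracks keep running in parallel, with a debug print of the new track.
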(event `self.ReceiveBeginPlay`
  (bind _output (`|GetArrayItem` (`self.MusicRefs`) (`self.SongToStart`)))
  (for _array_element (`self.TrackList`)
    (bind _returnvalue (`GameplayStatics.CreateSound2D` _array_element 1.0 1.0 0.0 null))
    (`KismetArrayLibrary.Array_Add` (`self.MusicRefs`) _returnvalue)
    (`AudioComponent.SetVolumeMultiplier` _returnvalue 0.0)
    (`AudioComponent.Play` _returnvalue 0.0))
  (`AudioComponent.SetVolumeMultiplier` _output (`self.Music Volume`))
  (set `self.CurrentMusicRef` _output))

(event `ChangeMusicTo`
  (params (IndexOfSongToPLay :type Integer))
  (bind _output (`|GetArrayItem` (`self.MusicRefs`) IndexOfSongToPLay))
  (`AudioComponent.SetVolumeMultiplier` (`self.CurrentMusicRef`) 0.0)
  (`AudioComponent.SetVolumeMultiplier` _output (`self.Music Volume`))
  (bind _output_get (set `self.CurrentMusicRef` _output))
  (`KismetSystemLibrary.PrintString` (`KismetStringLibrary.Concat_StrStr` "Music Playing" (`KismetSystemLibrary.GetDisplayName` _output_get))))

(fn `UserConstructionScript`)